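; BP_Enemy is an enemy that follows a path of six ordered waypoint actors and can be killed.
; Tick moves its StaticMesh, not the actor, toward TargetAtual at constant speed, picking the waypoint from CurrentPoint.
; CurrentPoint increments when the mesh gets close to the target, with no wrap after the last point.
; PerdeVida removes one point of Vida and calls MorteInimigo to destroy the actor when none remains.
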(event `self.ReceiveTick`
  (params (DeltaSeconds :type "Float (single-precision)"))
  (bind _returnvalue (`SceneComponent.K2_GetComponentLocation` (`self.StaticMesh`)))
  (bind _returnvalue_2 (`self.K2_GetActorLocation` (`self.TargetAtual`)))
  ;[1 1 1] Movimentação
  (`SceneComponent.K2_SetWorldLocation` (`self.StaticMesh`) (`KismetMathLibrary.VInterpTo_Constant` _returnvalue _returnvalue_2 DeltaSeconds 500.0) false false)
  (switch `int` (`self.CurrentPoint`)
    (:`1`
      (set `self.TargetAtual` (`self.Ponto01`)))
    (:`2`
      (set `self.TargetAtual` (`self.Ponto02`)))
    (:`3`
      (set `self.TargetAtual` (`self.Ponto03`)))
    (:`4`
      (set `self.TargetAtual` (`self.Ponto04`)))
    (:`5`
      (set `self.TargetAtual` (`self.Ponto05`)))
    (:`6`
      (set `self.TargetAtual` (`self.Ponto06`))))
  (if (< (`KismetMathLibrary.Vector_Distance` _returnvalue _returnvalue_2) 50.0)
    (bind _result (`/Engine/EditorBlueprintResources/StandardMacros.IncrementInt` (`self.CurrentPoint`))
      (:`  `
        (set `self.CurrentPoint` _result)))))

(event `MorteInimigo`
  ;[1 1 1] Morte do Inimigo
  (`self.K2_DestroyActor`))

(event `PerdeVida`
  ;[1 1 1] Tirando a vida do Inimigo
  (bind _result (`/Engine/EditorBlueprintResources/StandardMacros.DecrementInt` (`self.Vida`))
    (:`  `
      (set `self.Vida` _result)
      (if (< (`self.Vida`) 1)
        (`self.MorteInimigo`)))))

(fn `UserConstructionScript`)