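; BP_SpawnEnemy is a spawner that creates a set number of BP_Enemy actors at its own transform when play begins.
; Each spawn passes six Ponto points to the new enemy and always spawns regardless of collision.
; A counter tracks spawns, and the event re-calls itself after a one-second delay until the target count is reached.
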(event `self.ReceiveBeginPlay`
  (`self.Spawn Enemy`))

(event `Spawn Enemy`
  (`|SpawnActorFromClass` "/Game/MyGame/Inimigos/BP_Enemy.BP_Enemy_C" (`self.GetTransform`) "AlwaysSpawn" "MultiplyWithRoot" null (`self.Ponto01`) (`self.Ponto02`) (`self.Ponto03`) (`self.Ponto04`) (`self.Ponto05`) (`self.Ponto06`) null)
  (set `self.SpawnedEnimies` (+ (`self.SpawnedEnimies`) 1))
  (if (> (`self.EnimiesToSpawner`) (`self.SpawnedEnimies`))
    (`KismetSystemLibrary.Delay` 1.0)
    (`self.Spawn Enemy`)))

(fn `UserConstructionScript`)